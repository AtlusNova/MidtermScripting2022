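; EnemyCharacter is an enemy that chases characters it sees and kills the player on contact.
; PawnSensing's OnSeePawn sends it toward any seen Character with AIMoveTo, while an overlap with the player character sets FirstPersonPlayer Health to zero.
; It also carries axis input handlers for moving and looking.
; Disconnected CanSeeEnemy, delay and DoOnce nodes never run.
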(event `InputAxis|MoveForward`
  (params (AxisValue :type "Float (single-precision)"))
  ;[1 1 1] movement controller
  (`self.AddMovementInput` (`KismetMathLibrary.GetForwardVector` (`KismetMathLibrary.MakeRotator` 0.0 0.0 (.yaw (`self.GetControlRotation`)))) AxisValue))

(event `InputAxis|MoveRight`
  (params (AxisValue :type "Float (single-precision)"))
  ;[1 1 1] movement controller
  (`self.AddMovementInput` (`KismetMathLibrary.GetRightVector` (`KismetMathLibrary.MakeRotator` 0.0 0.0 (.yaw (`self.GetControlRotation`)))) AxisValue))

(event `InputAxis|Turn`
  (params (AxisValue :type "Float (single-precision)"))
  ;[1 1 1] movement controller
  (`self.AddControllerYawInput` AxisValue))

(event `InputAxis|LookUp`
  (params (AxisValue :type "Float (single-precision)"))
  ;[1 1 1] movement controller
  (`self.AddControllerPitchInput` AxisValue))

(event `self.ReceiveActorBeginOverlap`
  (params (OtherActor :type "Actor Object Reference"))
  (bind _returnvalue (`GameplayStatics.GetPlayerCharacter` 0))
  ;[1 1 1] kill player
  (if (`self.IsOverlappingActor` _returnvalue)
    (bind _asfirst_person_player (cast `/Game/Blueprints/FirstPersonPlayer` _returnvalue))
    (set `/Game/Blueprints/FirstPersonPlayer.Health` 0 _asfirst_person_player)))

(event `self.PawnSensing.OnSeePawn`
  (params (Pawn :type "Pawn Object Reference"))
  ;[1 1 1] chase player
  (bind _ascharacter (cast `Character` Pawn))
  (`|AIMoveTo` self (0.0 0.0 0.0) _ascharacter))

(fn `UserConstructionScript`)